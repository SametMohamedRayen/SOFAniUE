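; WebServiceApiHelper_BP is a Blueprint helper that watches for web service API responses and announces them to listeners.
; A custom event caches the current global response, and Tick compares it each frame against that cached value.
; When the value changes, it updates the cache and fires a response-received event dispatcher with the new value, skipping responses equal to "FAIL".
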(event `CustomEvent`
  (set `self.OldGlobalResponseValue` (`self.GetGlobalResponse`)))

(event `self.ReceiveTick`
  (params (DeltaSeconds :type "Float (single-precision)"))
  (`self.CheckValidResponseReceived`))

(fn `CheckValidResponseReceived`
  (bind _globalresponse (`self.GetGlobalResponse`))
  (if (not (`KismetStringLibrary.EqualEqual_StrStr` (`self.OldGlobalResponseValue`) _globalresponse))
    (set `self.OldGlobalResponseValue` _globalresponse)
    (if (not (`KismetStringLibrary.EqualEqual_StrStr` (`self.GetGlobalResponse`) "FAIL"))
      (`self.ResponseReceivedEventDispatcher` (`self.GetGlobalResponse`)))))

(fn `UserConstructionScript`)