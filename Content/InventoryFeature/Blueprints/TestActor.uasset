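; Test actor that builds a mesh at runtime from an FBX file embedded as a Base64 string, a cube exported from Blender.
; On BeginPlay, BinaryDataHelper imports the string using the Mesh component, which is then scaled up and raised vertically.
; A disconnected debug loop would print the helper's parsed normal values, but it never runs.
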(event `self.ReceiveBeginPlay`
  (bind _mesh (`self.Mesh`))
  (`BinaryDataHelper.ImportMeshFromBase64` (`self.BinaryDataHelper`) "S2F5ZGFyYSBGQlggQmluYXJ5ICAAGgDoHAAAlgcAAAAAAAAAAAAAEkZCWEhlYWRlckV4dGVuc2lvblwAAAABAAAABQAAABBGQlhIZWFkZXJWZXJzaW9uSesDAAB4AAAAAQAAAAUAAAAKRkJYVmVyc2lvbknoHAAAmAAAAAEAAAAFAAAADkVuY3J5cHRpb25UeXBlSQAAAACBAQAAAAAAAAAAAAARQ3JlYXRpb25UaW1lU3RhbXDPAAAAAQAAAAUAAAAHVmVyc2lvbknoAwAA5QAAAAEAAAAFAAAABFllYXJJ5wcAAPwAAAABAAAABQAAAAVNb250aEkEAAAAEQEAAAEAAAAFAAAAA0RheUkZAAAAJwEAAAEAAAAFAAAABEhvdXJJDQAAAD8BAAABAAAABQAAAAZNaW51dGVJBAAAAFcBAAABAAAABQAAAAZTZWNvbmRJLQAAAHQBAAABAAAABQAAAAtNaWxsaXNlY29uZEmUAAAAAAAAAAAAAAAAAAAAAMIBAAABAAAALQAAAAdDcmVhdG9yUygAAABCbGVuZGVyIChzdGFibGUgRkJYIElPKSAtIDMuMy4wIC0gNC4zNi4ziQcAAAIAAAAnAAAACVNjZW5lSW5mb1MVAAAAR2xvYmFsSW5mbwABU2NlbmVJbmZvUwgAAABVc2VyRGF0YR0CAAABAAAADQAAAARUeXBlUwgAAABVc2VyRGF0YTYCAAABAAAABQAAAAdWZXJzaW9uSWQAAAAGAwAAAAAAAAAAAAAITWV0YURhdGFkAgAAAQAAAAUAAAAHVmVyc2lvbklkAAAAewIAAAEAAAAFAAAABVRpdGxlUwAAAACUAgAAAQAAAAUAAAAHU3ViamVjdFMAAAAArAIAAAEAAAAFAAAABkF1dGhvclMAAAAAxgIAAAEAAAAFAAAACEtleXdvcmRzUwAAAADgAgAAAQAAAAUAAAAIUmV2aXNpb25TAAAAAPkCAAABAAAABQAAAAdDb21tZW50UwAAAAAAAAAAAAAAAAAAAAAAfAcAAAAAAAAAAAAADFByb3BlcnRpZXM3MGYDAAAFAAAAOQAAAAFQUwsAAABEb2N1bWVudFVybFMHAAAAS1N0cmluZ1MDAAAAVXJsUwAAAABTCwAAAC9mb29iYXIuZmJ4sAMAAAUAAAA8AAAAAVBTDgAAAFNyY0RvY3VtZW50VXJsUwcAAABLU3RyaW5nUwMAAABVcmxTAAAAAFMLAAAAL2Zvb2Jhci5mYnjiAwAABAAAACQAAAABUFMIAAAAT3JpZ2luYWxTCAAAAENvbXBvdW5kUwAAAABTAAAAADwEAAAFAAAATAAAAAFQUxoAAABPcmlnaW5hbHxBcHBsaWNhdGlvblZlbmRvclMHAAAAS1N0cmluZ1MAAAAAUwAAAABTEgAAAEJsZW5kZXIgRm91bmRhdGlvbpkEAAAFAAAATwAAAAFQUxgAAABPcmlnaW5hbHxBcHBsaWNhdGlvbk5hbWVTBwAAAEtTdHJpbmdTAAAAAFMAAAAAUxcAAABCbGVuZGVyIChzdGFibGUgRkJYIElPKecEAAAFAAAAQAAAAAFQUxsAAABPcmlnaW5hbHxBcHBsaWNhdGlvblZlcnNpb25TBwAAAEtTdHJpbmdTAAAAAFMAAAAAUwUAAAAzLjMuMEIFAAAFAAAATQAAAAFQUxUAAABPcmlnaW5hbHxEYXRlVGltZV9HTVRTCAAAAERhdGVUaW1lUwAAAABTAAAAAFMXAAAAMDEvMDEvMTk3MCAwMDowMDowMC4wMDCMBQAABQAAADwAAAABUFMRAAAAT3JpZ2luYWx8RmlsZU5hbWVTBwAAAEtTdHJpbmdTAAAAAFMAAAAAUwsAAAAvZm9vYmFyLmZieL8FAAAEAAAAJQAAAAFQUwkAAABMYXN0U2F2ZWRTCAAAAENvbXBvdW5kUwAAAABTAAAAABoGAAAFAAAATQAAAAFQUxsAAABMYXN0U2F2ZWR8QXBwbGljYXRpb25WZW5kb3JTBwAAAEtTdHJpbmdTAAAAAFMAAAAAUxIAAABCbGVuZGVyIEZvdW5kYXRpb254BgAABQAAAFAAAAABUFMZAAAATGFzdFNhdmVkfEFwcGxpY2F0aW9uTmFtZVMHAAAAS1N0cmluZ1MAAAAAUwAAAABTFwAAAEJsZW5kZXIgKHN0YWJsZSBGQlggSU8pxwYAAAUAAABBAAAAAVBTHAAAAExhc3RTYXZlZHxBcHBsaWNhdGlvblZlcnNpb25TBwAAAEtTdHJpbmdTAAAAAFMAAAAAUwUAAAAzLjMuMCMHAAAFAAAATgAAAAFQUxYAAABMYXN0U2F2ZWR8RGF0ZVRpbWVfR01UUwgAAABEYXRlVGltZVMAAAAAUwAAAABTFwAAADAxLzAxLzE5NzAgMDA6MDA6MDAuMDAwbwcAAAUAAAA+AAAAAVBTHgAAAE9yaWdpbmFsfEFwcGxpY2F0aW9uTmF0aXZlRmlsZVMHAAAAS1N0cmluZ1MAAAAAUwAAAABTAAAAAAAAAAAAAAAAAAAAAAAAAAAAAAAAAAAAAAAAAAAAAAAAAAAAAAAAAL4HAAABAAAAFQAAAAZGaWxlSWRSEAAAACizKuu2JMzCv8iwKqkr/PHzBwAAAQAAABwAAAAMQ3JlYXRpb25UaW1lUxcAAAAxOTcwLTAxLTAxIDEwOjAwOjAwOjAwMDQIAAABAAAALQAAAAdDcmVhdG9yUygAAABCbGVuZGVyIChzdGFibGUgRkJYIElPKSAtIDMuMy4wIC0gNC4zNi4zsgwAAAAAAAAAAAAADkdsb2JhbFNldHRpbmdzaAgAAAEAAAAFAAAAB1ZlcnNpb25J6AMAAKUMAAAAAAAAAAAAAAxQcm9wZXJ0aWVzNzC4CAAABQAAACkAAAABUFMGAAAAVXBBeGlzUwMAAABpbnRTBwAAAEludGVnZXJTAAAAAEkBAAAA8wgAAAUAAAAtAAAAAVBTCgAAAFVwQXhpc1NpZ25TAwAAAGludFMHAAAASW50ZWdlclMAAAAASQEAAAAtCQAABQAAACwAAAABUFMJAAAARnJvbnRBeGlzUwMAAABpbnRTBwAAAEludGVnZXJTAAAAAEkCAAAAawkAAAUAAAAwAAAAAVBTDQAAAEZyb250QXhpc1NpZ25TAwAAAGludFMHAAAASW50ZWdlclMAAAAASQEAAAClCQAABQAAACwAAAABUFMJAAAAQ29vcmRBeGlzUwMAAABpbnRTBwAAAEludGVnZXJTAAAAAEkAAAAA4wkAAAUAAAAwAAAAAVBTDQAAAENvb3JkQXhpc1NpZ25TAwAAAGludFMHAAAASW50ZWdlclMAAAAASQEAAAAiCgAABQAAADEAAAABUFMOAAAAT3JpZ2luYWxVcEF4aXNTAwAAAGludFMHAAAASW50ZWdlclMAAAAASf////9lCgAABQAAADUAAAABUFMSAAAAT3JpZ2luYWxVcEF4aXNTaWduUwMAAABpbnRTBwAAAEludGVnZXJTAAAAAEkBAAAAqwoAAAUAAAA4AAAAAVBTDwAAAFVuaXRTY2FsZUZhY3RvclMGAAAAZG91YmxlUwYAAABOdW1iZXJTAAAAAEQAAAAAAADwP/kKAAAFAAAAQAAAAAFQUxcAAABPcmlnaW5hbFVuaXRTY2FsZUZhY3RvclMGAAAAZG91YmxlUwYAAABOdW1iZXJTAAAAAEQAAAAAAADwP08LAAAHAAAASAAAAAFQUwwAAABBbWJpZW50Q29sb3JTCAAAAENvbG9yUkdCUwUAAABDb2xvclMAAAAARAAAAAAAAAAARAAAAAAAAAAARAAAAAAAAAAAngsAAAUAAABBAAAAAVBTDQAAAERlZmF1bHRDYW1lcmFTBwAAAEtTdHJpbmdTAAAAAFMAAAAAUxQAAABQcm9kdWNlciBQZXJzcGVjdGl2ZdELAAAFAAAAJQAAAAFQUwgAAABUaW1lTW9kZVMEAAAAZW51bVMAAAAAUwAAAABJCwAAABIMAAAFAAAAMwAAAAFQUw0AAABUaW1lU3BhblN0YXJ0UwUAAABLVGltZVMEAAAAVGltZVMAAAAATAAAAAAAAAAAUgwAAAUAAAAyAAAAAVBTDAAAAFRpbWVTcGFuU3RvcFMFAAAAS1RpbWVTBAAAAFRpbWVTAAAAAEyw1+jACgAAAJgMAAAFAAAAOAAAAAFQUw8AAABDdXN0b21GcmFtZVJhdGVTBgAAAGRvdWJsZVMGAAAATnVtYmVyUwAAAABEAAAAAAAAOEAAAAAAAAAAAAAAAAAAAAAAAAAAAAAAAAAAAOQNAAAAAAAAAAAAAAlEb2N1bWVudHPfDAAAAQAAAAUAAAAFQ291bnRJAQAAANcNAAADAAAAHQAAAAhEb2N1bWVudEyvGU4LAAAAAFMFAAAAU2NlbmVTBQAAAFNjZW5lrA0AAAAAAAAAAAAADFByb3BlcnRpZXM3MF4NAAAEAAAAJgAAAAFQUwwAAABTb3VyY2VPYmplY3RTBgAAAG9iamVjdFMAAAAAUwAAAACfDQAABQAAADMAAAABUFMTAAAAQWN0aXZlQW5pbVN0YWNrTmFtZVMHAAAAS1N0cmluZ1MAAAAAUwAAAABTAAAAAAAAAAAAAAAAAAAAAADKDQAAAQAAAAkAAAAIUm9vdE5vZGVMAAAAAAAAAAAAAAAAAAAAAAAAAAAAAAAAAAAAAAAAAAAAAAgOAAAAAAAAAAAAAApSZWZlcmVuY2VzAAAAAAAAAAAAAAAAAAosAAAAAAAAAAAAAAtEZWZpbml0aW9uczkOAAABAAAABQAAAAdWZXJzaW9uSWQAAABQDgAAAQAAAAUAAAAFQ291bnRJBAAAAJ4OAAABAAAAEwAAAApPYmplY3RUeXBlUw4AAABHbG9iYWxTZXR0aW5nc5EOAAABAAAABQAAAAVDb3VudEkBAAAAAAAAAAAAAAAAAAAAAOQQAAABAAAADQAAAApPYmplY3RUeXBlUwgAAABHZW9tZXRyedkOAAABAAAABQAAAAVDb3VudEkBAAAA1xAAAAEAAAAMAAAAEFByb3BlcnR5VGVtcGxhdGVTBwAAAEZieE1lc2jKEAAAAAAAAAAAAAAMUHJvcGVydGllczcwag8AAAcAAABBAAAAAVBTBQAAAENvbG9yUwgAAABDb2xvclJHQlMFAAAAQ29sb3JTAAAAAESamZmZmZnpP0SamZmZmZnpP0SamZmZmZnpP7wPAAAHAAAARAAAAAFQUwcAAABCQm94TWluUwgAAABWZWN0b3IzRFMGAAAAVmVjdG9yUwAAAABEAAAAAAAAAABEAAAAAAAAAABEAAAAAAAAAAAOEAAABwAAAEQAAAABUFMHAAAAQkJveE1heFMIAAAAVmVjdG9yM0RTBgAAAFZlY3RvclMAAAAARAAAAAAAAAAARAAAAAAAAAAARAAAAAAAAAAASxAAAAUAAAAvAAAAAVBTEgAAAFByaW1hcnkgVmlzaWJpbGl0eVMEAAAAYm9vbFMAAAAAUwAAAABJAQAAAIMQAAAFAAAAKgAAAAFQUw0AAABDYXN0cyBTaGFkb3dzUwQAAABib29sUwAAAABTAAAAAEkBAAAAvRAAAAUAAAAsAAAAAVBTDwAAAFJlY2VpdmUgU2hhZG93c1MEAAAAYm9vbFMAAAAAUwAAAABJAQAAAAAAAAAAAAAAAAAAAAAAAAAAAAAAAAAAAAAAAAAAAAAAAAAAAAAAAIckAAABAAAACgAAAApPYmplY3RUeXBlUwUAAABNb2RlbBwRAAABAAAABQAAAAVDb3VudEkBAAAAeiQAAAEAAAAMAAAAEFByb3BlcnR5VGVtcGxhdGVTBwAAAEZieE5vZGVtJAAAAAAAAAAAAAAMUHJvcGVydGllczcwnhEAAAUAAAAyAAAAAVBTFQAAAFF1YXRlcm5pb25JbnRlcnBvbGF0ZVMEAAAAZW51bVMAAAAAUwAAAABJAAAAAPcRAAAHAAAASwAAAAFQUw4AAABSb3RhdGlvbk9mZnNldFMIAAAAVmVjdG9yM0RTBgAAAFZlY3RvclMAAAAARAAAAAAAAAAARAAAAAAAAAAARAAAAAAAAAAATxIAAAcAAABKAAAAAVBTDQAAAFJvdGF0aW9uUGl2b3RTCAAAAFZlY3RvcjNEUwYAAABWZWN0b3JTAAAAAEQAAAAAAAAAAEQAAAAAAAAAAEQAAAAAAAAAAKcSAAAHAAAASgAAAAFQUw0AAABTY2FsaW5nT2Zmc2V0UwgAAABWZWN0b3IzRFMGAAAAVmVjdG9yUwAAAABEAAAAAAAAAABEAAAAAAAAAABEAAAAAAAAAAD+EgAABwAAAEkAAAABUFMMAAAAU2NhbGluZ1Bpdm90UwgAAABWZWN0b3IzRFMGAAAAVmVjdG9yUwAAAABEAAAAAAAAAABEAAAAAAAAAABEAAAAAAAAAAA6EwAABQAAAC4AAAABUFMRAAAAVHJhbnNsYXRpb25BY3RpdmVTBAAAAGJvb2xTAAAAAFMAAAAASQAAAACTEwAABwAAAEsAAAABUFMOAAAAVHJhbnNsYXRpb25NaW5TCAAAAFZlY3RvcjNEUwYAAABWZWN0b3JTAAAAAEQAAAAAAAAAAEQAAAAAAAAAAEQAAAAAAAAAAOwTAAAHAAAASwAAAAFQUw4AAABUcmFuc2xhdGlvbk1heFMIAAAAVmVjdG9yM0RTBgAAAFZlY3RvclMAAAAARAAAAAAAAAAARAAAAAAAAAAARAAAAAAAAAAAJhQAAAUAAAAsAAAAAVBTDwAAAFRyYW5zbGF0aW9uTWluWFMEAAAAYm9vbFMAAAAAUwAAAABJAAAAAGAUAAAFAAAALAAAAAFQUw8AAABUcmFuc2xhdGlvbk1pbllTBAAAAGJvb2xTAAAAAFMAAAAASQAAAACaFAAABQAAACwAAAABUFMPAAAAVHJhbnNsYXRpb25NaW5aUwQAAABib29sUwAAAABTAAAAAEkAAAAA1BQAAAUAAAAsAAAAAVBTDwAAAFRyYW5zbGF0aW9uTWF4WFMEAAAAYm9vbFMAAAAAUwAAAABJAAAAAA4VAAAFAAAALAAAAAFQUw8AAABUcmFuc2xhdGlvbk1heFlTBAAAAGJvb2xTAAAAAFMAAAAASQAAAABIFQAABQAAACwAAAABUFMPAAAAVHJhbnNsYXRpb25NYXhaUwQAAABib29sUwAAAABTAAAAAEkAAAAAgBUAAAUAAAAqAAAAAVBTDQAAAFJvdGF0aW9uT3JkZXJTBAAAAGVudW1TAAAAAFMAAAAASQAAAADEFQAABQAAADYAAAABUFMZAAAAUm90YXRpb25TcGFjZUZvckxpbWl0T25seVMEAAAAYm9vbFMAAAAAUwAAAABJAAAAAA0WAAAFAAAAOwAAAAFQUxIAAABSb3RhdGlvblN0aWZmbmVzc1hTBgAAAGRvdWJsZVMGAAAATnVtYmVyUwAAAABEAAAAAAAAAABWFgAABQAAADsAAAABUFMSAAAAUm90YXRpb25TdGlmZm5lc3NZUwYAAABkb3VibGVTBgAAAE51bWJlclMAAAAARAAAAAAAAAAAnxYAAAUAAAA7AAAAAVBTEgAAAFJvdGF0aW9uU3RpZmZuZXNzWlMGAAAAZG91YmxlUwYAAABOdW1iZXJTAAAAAEQAAAAAAAAAAN0WAAAFAAAAMAAAAAFQUwcAAABBeGlzTGVuUwYAAABkb3VibGVTBgAAAE51bWJlclMAAAAARAAAAAAAACRAMxcAAAcAAABIAAAAAVBTCwAAAFByZVJvdGF0aW9uUwgAAABWZWN0b3IzRFMGAAAAVmVjdG9yUwAAAABEAAAAAAAAAABEAAAAAAAAAABEAAAAAAAAAACKFwAABwAAAEkAAAABUFMMAAAAUG9zdFJvdGF0aW9uUwgAAABWZWN0b3IzRFMGAAAAVmVjdG9yUwAAAABEAAAAAAAAAABEAAAAAAAAAABEAAAAAAAAAADDFwAABQAAACsAAAABUFMOAAAAUm90YXRpb25BY3RpdmVTBAAAAGJvb2xTAAAAAFMAAAAASQAAAAAZGAAABwAAAEgAAAABUFMLAAAAUm90YXRpb25NaW5TCAAAAFZlY3RvcjNEUwYAAABWZWN0b3JTAAAAAEQAAAAAAAAAAEQAAAAAAAAAAEQAAAAAAAAAAG8YAAAHAAAASAAAAAFQUwsAAABSb3RhdGlvbk1heFMIAAAAVmVjdG9yM0RTBgAAAFZlY3RvclMAAAAARAAAAAAAAAAARAAAAAAAAAAARAAAAAAAAAAAphgAAAUAAAApAAAAAVBTDAAAAFJvdGF0aW9uTWluWFMEAAAAYm9vbFMAAAAAUwAAAABJAAAAAN0YAAAFAAAAKQAAAAFQUwwAAABSb3RhdGlvbk1pbllTBAAAAGJvb2xTAAAAAFMAAAAASQAAAAAUGQAABQAAACkAAAABUFMMAAAAUm90YXRpb25NaW5aUwQAAABib29sUwAAAABTAAAAAEkAAAAASxkAAAUAAAApAAAAAVBTDAAAAFJvdGF0aW9uTWF4WFMEAAAAYm9vbFMAAAAAUwAAAABJAAAAAIIZAAAFAAAAKQAAAAFQUwwAAABSb3RhdGlvbk1heFlTBAAAAGJvb2xTAAAAAFMAAAAASQAAAAC5GQAABQAAACkAAAABUFMMAAAAUm90YXRpb25NYXhaUwQAAABib29sUwAAAABTAAAAAEkAAAAA7xkAAAUAAAAoAAAAAVBTCwAAAEluaGVyaXRUeXBlUwQAAABlbnVtUwAAAABTAAAAAEkAAAAAJxoAAAUAAAAqAAAAAVBTDQAAAFNjYWxpbmdBY3RpdmVTBAAAAGJvb2xTAAAAAFMAAAAASQAAAAB8GgAABwAAAEcAAAABUFMKAAAAU2NhbGluZ01pblMIAAAAVmVjdG9yM0RTBgAAAFZlY3RvclMAAAAARAAAAAAAAAAARAAAAAAAAAAARAAAAAAAAAAA0RoAAAcAAABHAAAAAVBTCgAAAFNjYWxpbmdNYXhTCAAAAFZlY3RvcjNEUwYAAABWZWN0b3JTAAAAAEQAAAAAAADwP0QAAAAAAADwP0QAAAAAAADwPwcbAAAFAAAAKAAAAAFQUwsAAABTY2FsaW5nTWluWFMEAAAAYm9vbFMAAAAAUwAAAABJAAAAAD0bAAAFAAAAKAAAAAFQUwsAAABTY2FsaW5nTWluWVMEAAAAYm9vbFMAAAAAUwAAAABJAAAAAHMbAAAFAAAAKAAAAAFQUwsAAABTY2FsaW5nTWluWlMEAAAAYm9vbFMAAAAAUwAAAABJAAAAAKkbAAAFAAAAKAAAAAFQUwsAAABTY2FsaW5nTWF4WFMEAAAAYm9vbFMAAAAAUwAAAABJAAAAAN8bAAAFAAAAKAAAAAFQUwsAAABTY2FsaW5nTWF4WVMEAAAAYm9vbFMAAAAAUwAAAABJAAAAABUcAAAFAAAAKAAAAAFQUwsAAABTY2FsaW5nTWF4WlMEAAAAYm9vbFMAAAAAUwAAAABJAAAAAHQcAAAHAAAAUQAAAAFQUxQAAABHZW9tZXRyaWNUcmFuc2xhdGlvblMIAAAAVmVjdG9yM0RTBgAAAFZlY3RvclMAAAAARAAAAAAAAAAARAAAAAAAAAAARAAAAAAAAAAA0BwAAAcAAABOAAAAAVBTEQAAAEdlb21ldHJpY1JvdGF0aW9uUwgAAABWZWN0b3IzRFMGAAAAVmVjdG9yUwAAAABEAAAAAAAAAABEAAAAAAAAAABEAAAAAAAAAAArHQAABwAAAE0AAAABUFMQAAAAR2VvbWV0cmljU2NhbGluZ1MIAAAAVmVjdG9yM0RTBgAAAFZlY3RvclMAAAAARAAAAAAAAPA/RAAAAAAAAPA/RAAAAAAAAPA/bx0AAAUAAAA2AAAAAVBTDQAAAE1pbkRhbXBSYW5nZVhTBgAAAGRvdWJsZVMGAAAATnVtYmVyUwAAAABEAAAAAAAAAACzHQAABQAAADYAAAABUFMNAAAATWluRGFtcFJhbmdlWVMGAAAAZG91YmxlUwYAAABOdW1iZXJTAAAAAEQAAAAAAAAAAPcdAAAFAAAANgAAAAFQUw0AAABNaW5EYW1wUmFuZ2VaUwYAAABkb3VibGVTBgAAAE51bWJlclMAAAAARAAAAAAAAAAAOx4AAAUAAAA2AAAAAVBTDQAAAE1heERhbXBSYW5nZVhTBgAAAGRvdWJsZVMGAAAATnVtYmVyUwAAAABEAAAAAAAAAAB/HgAABQAAADYAAAABUFMNAAAATWF4RGFtcFJhbmdlWVMGAAAAZG91YmxlUwYAAABOdW1iZXJTAAAAAEQAAAAAAAAAAMMeAAAFAAAANgAAAAFQUw0AAABNYXhEYW1wUmFuZ2VaUwYAAABkb3VibGVTBgAAAE51bWJlclMAAAAARAAAAAAAAAAACh8AAAUAAAA5AAAAAVBTEAAAAE1pbkRhbXBTdHJlbmd0aFhTBgAAAGRvdWJsZVMGAAAATnVtYmVyUwAAAABEAAAAAAAAAABRHwAABQAAADkAAAABUFMQAAAATWluRGFtcFN0cmVuZ3RoWVMGAAAAZG91YmxlUwYAAABOdW1iZXJTAAAAAEQAAAAAAAAAAJgfAAAFAAAAOQAAAAFQUxAAAABNaW5EYW1wU3RyZW5ndGhaUwYAAABkb3VibGVTBgAAAE51bWJlclMAAAAARAAAAAAAAAAA3x8AAAUAAAA5AAAAAVBTEAAAAE1heERhbXBTdHJlbmd0aFhTBgAAAGRvdWJsZVMGAAAATnVtYmVyUwAAAABEAAAAAAAAAAAmIAAABQAAADkAAAABUFMQAAAATWF4RGFtcFN0cmVuZ3RoWVMGAAAAZG91YmxlUwYAAABOdW1iZXJTAAAAAEQAAAAAAAAAAG0gAAAFAAAAOQAAAAFQUxAAAABNYXhEYW1wU3RyZW5ndGhaUwYAAABkb3VibGVTBgAAAE51bWJlclMAAAAARAAAAAAAAAAAsiAAAAUAAAA3AAAAAVBTDgAAAFByZWZlcmVkQW5nbGVYUwYAAABkb3VibGVTBgAAAE51bWJlclMAAAAARAAAAAAAAAAA9yAAAAUAAAA3AAAAAVBTDgAAAFByZWZlcmVkQW5nbGVZUwYAAABkb3VibGVTBgAAAE51bWJlclMAAAAARAAAAAAAAAAAPCEAAAUAAAA3AAAAAVBTDgAAAFByZWZlcmVkQW5nbGVaUwYAAABkb3VibGVTBgAAAE51bWJlclMAAAAARAAAAAAAAAAAciEAAAQAAAAoAAAAAVBTDgAAAExvb2tBdFByb3BlcnR5UwYAAABvYmplY3RTAAAAAFMAAAAAqiEAAAQAAAAqAAAAAVBTEAAAAFVwVmVjdG9yUHJvcGVydHlTBgAAAG9iamVjdFMAAAAAUwAAAADZIQAABQAAACEAAAABUFMEAAAAU2hvd1MEAAAAYm9vbFMAAAAAUwAAAABJAQAAAB8iAAAFAAAAOAAAAAFQUxsAAABOZWdhdGl2ZVBlcmNlbnRTaGFwZVN1cHBvcnRTBAAAAGJvb2xTAAAAAFMAAAAASQEAAABlIgAABQAAADgAAAABUFMVAAAARGVmYXVsdEF0dHJpYnV0ZUluZGV4UwMAAABpbnRTBwAAAEludGVnZXJTAAAAAEn/////liIAAAUAAAAjAAAAAVBTBgAAAEZyZWV6ZVMEAAAAYm9vbFMAAAAAUwAAAABJAAAAAMciAAAFAAAAIwAAAAFQUwYAAABMT0RCb3hTBAAAAGJvb2xTAAAAAFMAAAAASQAAAAAjIwAABwAAAE4AAAABUFMPAAAATGNsIFRyYW5zbGF0aW9uUw8AAABMY2wgVHJhbnNsYXRpb25TAAAAAFMBAAAAQUQAAAAAAAAAAEQAAAAAAAAAAEQAAAAAAAAAAHkjAAAHAAAASAAAAAFQUwwAAABMY2wgUm90YXRpb25TDAAAAExjbCBSb3RhdGlvblMAAAAAUwEAAABBRAAAAAAAAAAARAAAAAAAAAAARAAAAAAAAAAAzSMAAAcAAABGAAAAAVBTCwAAAExjbCBTY2FsaW5nUwsAAABMY2wgU2NhbGluZ1MAAAAAUwEAAABBRAAAAAAAAPA/RAAAAAAAAPA/RAAAAAAAAPA/DSQAAAUAAAAyAAAAAVBTCgAAAFZpc2liaWxpdHlTCgAAAFZpc2liaWxpdHlTAAAAAFMBAAAAQUQAAAAAAADwP2AkAAAFAAAARQAAAAFQUxYAAABWaXNpYmlsaXR5IEluaGVyaXRhbmNlUxYAAABWaXNpYmlsaXR5IEluaGVyaXRhbmNlUwAAAABTAAAAAEkBAAAAAAAAAAAAAAAAAAAAAAAAAAAAAAAAAAAAAAAAAAAAAAAAAAAAAAAA/SsAAAEAAAANAAAACk9iamVjdFR5cGVTCAAAAE1hdGVyaWFswiQAAAEAAAAFAAAABUNvdW50SQEAAADwKwAAAQAAABQAAAAQUHJvcGVydHlUZW1wbGF0ZVMPAAAARmJ4U3VyZmFjZVBob25n4ysAAAAAAAAAAAAADFByb3BlcnRpZXM3MEslAAAFAAAAMQAAAAFQUwwAAABTaGFkaW5nTW9kZWxTBwAAAEtTdHJpbmdTAAAAAFMAAAAAUwUAAABQaG9uZ4AlAAAFAAAAJwAAAAFQUwoAAABNdWx0aUxheWVyUwQAAABib29sUwAAAABTAAAAAEkAAAAA0CUAAAcAAABCAAAAAVBTDQAAAEVtaXNzaXZlQ29sb3JTBQAAAENvbG9yUwAAAABTAQAAAEFEAAAAAAAAAABEAAAAAAAAAABEAAAAAAAAAAAQJgAABQAAADIAAAABUFMOAAAARW1pc3NpdmVGYWN0b3JTBgAAAE51bWJlclMAAAAAUwEAAABBRAAAAAAAAPA/XyYAAAcAAABBAAAAAVBTDAAAAEFtYmllbnRDb2xvclMFAAAAQ29sb3JTAAAAAFMBAAAAQUSamZmZmZnJP0SamZmZmZnJP0SamZmZmZnJP54mAAAFAAAAMQAAAAFQUw0AAABBbWJpZW50RmFjdG9yUwYAAABOdW1iZXJTAAAAAFMBAAAAQUQAAAAAAADwP+0mAAAHAAAAQQAAAAFQUwwAAABEaWZmdXNlQ29sb3JTBQAAAENvbG9yUwAAAABTAQAAAEFEmpmZmZmZ6T9EmpmZmZmZ6T9EmpmZmZmZ6T8sJwAABQAAADEAAAABUFMNAAAARGlmZnVzZUZhY3RvclMGAAAATnVtYmVyUwAAAABTAQAAAEFEAAAAAAAA8D9/JwAABwAAAEUAAAABUFMQAAAAVHJhbnNwYXJlbnRDb2xvclMFAAAAQ29sb3JTAAAAAFMBAAAAQUQAAAAAAAAAAEQAAAAAAAAAAEQAAAAAAAAAAMMnAAAFAAAANgAAAAFQUxIAAABUcmFuc3BhcmVuY3lGYWN0b3JTBgAAAE51bWJlclMAAAAAUwEAAABBRAAAAAAAAAAA/CcAAAUAAAArAAAAAVBTBwAAAE9wYWNpdHlTBgAAAE51bWJlclMAAAAAUwEAAABBRAAAAAAAAPA/UCgAAAcAAABGAAAAAVBTCQAAAE5vcm1hbE1hcFMIAAAAVmVjdG9yM0RTBgAAAFZlY3RvclMAAAAARAAAAAAAAAAARAAAAAAAAAAARAAAAAAAAAAAnygAAAcAAABBAAAAAVBTBAAAAEJ1bXBTCAAAAFZlY3RvcjNEUwYAAABWZWN0b3JTAAAAAEQAAAAAAAAAAEQAAAAAAAAAAEQAAAAAAAAAAOAoAAAFAAAAMwAAAAFQUwoAAABCdW1wRmFjdG9yUwYAAABkb3VibGVTBgAAAE51bWJlclMAAAAARAAAAAAAAPA/OykAAAcAAABNAAAAAVBTEQAAAERpc3BsYWNlbWVudENvbG9yUwgAAABDb2xvclJHQlMFAAAAQ29sb3JTAAAAAEQAAAAAAAAAAEQAAAAAAAAAAEQAAAAAAAAAAIQpAAAFAAAAOwAAAAFQUxIAAABEaXNwbGFjZW1lbnRGYWN0b3JTBgAAAGRvdWJsZVMGAAAATnVtYmVyUwAAAABEAAAAAAAA8D/lKQAABwAAAFMAAAABUFMXAAAAVmVjdG9yRGlzcGxhY2VtZW50Q29sb3JTCAAAAENvbG9yUkdCUwUAAABDb2xvclMAAAAARAAAAAAAAAAARAAAAAAAAAAARAAAAAAAAAAANCoAAAUAAABBAAAAAVBTGAAAAFZlY3RvckRpc3BsYWNlbWVudEZhY3RvclMGAAAAZG91YmxlUwYAAABOdW1iZXJTAAAAAEQAAAAAAADwP4QqAAAHAAAAQgAAAAFQUw0AAABTcGVjdWxhckNvbG9yUwUAAABDb2xvclMAAAAAUwEAAABBRJqZmZmZmck/RJqZmZmZmck/RJqZmZmZmck/xCoAAAUAAAAyAAAAAVBTDgAAAFNwZWN1bGFyRmFjdG9yUwYAAABOdW1iZXJTAAAAAFMBAAAAQUQAAAAAAADwP/8qAAAFAAAALQAAAAFQUwkAAABTaGluaW5lc3NTBgAAAE51bWJlclMAAAAAUwEAAABBRAAAAAAAADRAQisAAAUAAAA1AAAAAVBTEQAAAFNoaW5pbmVzc0V4cG9uZW50UwYAAABOdW1iZXJTAAAAAFMBAAAAQUQAAAAAAAA0QJQrAAAHAAAARAAAAAFQUw8AAABSZWZsZWN0aW9uQ29sb3JTBQAAAENvbG9yUwAAAABTAQAAAEFEAAAAAAAAAABEAAAAAAAAAABEAAAAAAAAAADWKwAABQAAADQAAAABUFMQAAAAUmVmbGVjdGlvbkZhY3RvclMGAAAATnVtYmVyUwAAAABTAQAAAEFEAAAAAAAA8D8AAAAAAAAAAAAAAAAAAAAAAAAAAAAAAAAAAAAAAAAAAAAAAAAAAAAAAAAAAAAAAAAAAAAAsTgAAAAAAAAAAAAAB09iamVjdHMJMwAAAwAAACUAAAAIR2VvbWV0cnlMzxw0BwAAAABTDgAAAEN1YmUAAUdlb21ldHJ5UwQAAABNZXNofiwAAAAAAAAAAAAADFByb3BlcnRpZXM3MAAAAAAAAAAAAAAAAACfLAAAAQAAAAUAAAAPR2VvbWV0cnlWZXJzaW9uSXwAAADqLAAAAQAAADYAAAAIVmVydGljZXNkGAAAAAEAAAApAAAAeAFjYACBD/ZgijC9H00dOh9mDkwcnYbJw2iYPDofJg6jccoDAO+tIml2LQAAAQAAAG0AAAASUG9seWdvblZlcnRleEluZGV4aRgAAAAAAAAAYAAAAAAAAAAEAAAABgAAAP3///8DAAAAAgAAAAYAAAD4////BwAAAAYAAAAEAAAA+v///wUAAAABAAAAAwAAAPj///8BAAAAAAAAAAIAAAD8////BQAAAAQAAAAAAAAA/v///8UtAAABAAAAPQAAAAVFZGdlc2kMAAAAAAAAADAAAAAAAAAAAQAAAAIAAAADAAAABAAAAAYAAAAHAAAACgAAAAsAAAAMAAAADQAAABAAAADiLgAAAQAAAAUAAAASTGF5ZXJFbGVtZW50Tm9ybWFsSQAAAAACLgAAAQAAAAUAAAAHVmVyc2lvbkllAAAAGC4AAAEAAAAFAAAABE5hbWVTAAAAAE8uAAABAAAAFAAAABZNYXBwaW5nSW5mb3JtYXRpb25UeXBlUw8AAABCeVBvbHlnb25WZXJ0ZXh/LgAAAQAAAAsAAAAYUmVmZXJlbmNlSW5mb3JtYXRpb25UeXBlUwYAAABEaXJlY3TVLgAAAQAAAEIAAAAHTm9ybWFsc2RIAAAAAQAAADUAAAB4AWNgwAY+2GMTZWCgVPzDfhzmUihOK3OxuxYYDhS6F2YuzBxKwxVuHo54IyRPvv0AiNEiaQAAAAAAAAAAAAAAAACUMAAAAQAAAAUAAAAOTGF5ZXJFbGVtZW50VVZJAAAAABsvAAABAAAABQAAAAdWZXJzaW9uSWUAAAA2LwAAAQAAAAoAAAAETmFtZVMFAAAAVVZNYXBtLwAAAQAAABQAAAAWTWFwcGluZ0luZm9ybWF0aW9uVHlwZVMPAAAAQnlQb2x5Z29uVmVydGV4pC8AAAEAAAASAAAAGFJlZmVyZW5jZUluZm9ybWF0aW9uVHlwZVMNAAAASW5kZXhUb0RpcmVjdAYwAAABAAAAUwAAAAJVVmQcAAAAAQAAAEYAAAB4AV2NoREAIAwDs1lXZwQkEoFAIBiBA/KmNbm/pIl0b8QTbStczc3arSsx+Zny9PGPT/6vSviZ2S9pj3368GH6exy0Qh0LhzAAAAEAAABtAAAAB1VWSW5kZXhpGAAAAAAAAABgAAAADQAAAAMAAAALAAAABAAAAAYAAAAEAAAAAAAAAAUAAAAIAAAABwAAAAEAAAAJAAAACgAAAAIAAAAGAAAADAAAAAIAAAANAAAABAAAAAYAAAAJAAAAAQAAAA0AAAACAAAAAAAAAAAAAAAAAAAAAIMxAAABAAAABQAAABRMYXllckVsZW1lbnRNYXRlcmlhbEkAAAAA0zAAAAEAAAAFAAAAB1ZlcnNpb25JZQAAAOkwAAABAAAABQAAAAROYW1lUwAAAAAYMQAAAQAAAAwAAAAWTWFwcGluZ0luZm9ybWF0aW9uVHlwZVMHAAAAQWxsU2FtZU8xAAABAAAAEgAAABhSZWZlcmVuY2VJbmZvcm1hdGlvblR5cGVTDQAAAEluZGV4VG9EaXJlY3R2MQAAAQAAABEAAAAJTWF0ZXJpYWxzaQEAAAAAAAAABAAAAAAAAAAAAAAAAAAAAAAAAAAA/DIAAAEAAAAFAAAABUxheWVySQAAAACzMQAAAQAAAAUAAAAHVmVyc2lvbklkAAAAHTIAAAAAAAAAAAAADExheWVyRWxlbWVudPQxAAABAAAAFwAAAARUeXBlUxIAAABMYXllckVsZW1lbnROb3JtYWwQMgAAAQAAAAUAAAAKVHlwZWRJbmRleEkAAAAAAAAAAAAAAAAAAAAAAIMyAAAAAAAAAAAAAAxMYXllckVsZW1lbnRaMgAAAQAAABMAAAAEVHlwZVMOAAAATGF5ZXJFbGVtZW50VVZ2MgAAAQAAAAUAAAAKVHlwZWRJbmRleEkAAAAAAAAAAAAAAAAAAAAAAO8yAAAAAAAAAAAAAAxMYXllckVsZW1lbnTGMgAAAQAAABkAAAAEVHlwZVMUAAAATGF5ZXJFbGVtZW50TWF0ZXJpYWziMgAAAQAAAAUAAAAKVHlwZWRJbmRleEkAAAAAAAAAAAAAAAAAAAAAAAAAAAAAAAAAAAAAAAAAAAAAAAAAAAAAAAAAHzUAAAMAAAAiAAAABU1vZGVsTKWx8RkAAAAAUwsAAABDdWJlAAFNb2RlbFMEAAAATWVzaFYzAAABAAAABQAAAAdWZXJzaW9uSegAAACiNAAAAAAAAAAAAAAMUHJvcGVydGllczcwxTMAAAcAAABIAAAAAVBTDAAAAExjbCBSb3RhdGlvblMMAAAATGNsIFJvdGF0aW9uUwAAAABTAQAAAEFE0gUnJwCAVsBEAAAAAAAAAABEAAAAAAAAAAAZNAAABwAAAEYAAAABUFMLAAAATGNsIFNjYWxpbmdTCwAAAExjbCBTY2FsaW5nUwAAAABTAQAAAEFEAAAAAAAAWUBEAAAAAAAAWUBEAAAAAAAAWUBfNAAABQAAADgAAAABUFMVAAAARGVmYXVsdEF0dHJpYnV0ZUluZGV4UwMAAABpbnRTBwAAAEludGVnZXJTAAAAAEkAAAAAlTQAAAUAAAAoAAAAAVBTCwAAAEluaGVyaXRUeXBlUwQAAABlbnVtUwAAAABTAAAAAEkBAAAAAAAAAAAAAAAAAAAAAL40AAABAAAABQAAAApNdWx0aUxheWVySQAAAADZNAAAAQAAAAUAAAAJTXVsdGlUYWtlSQAAAADvNAAAAQAAAAIAAAAHU2hhZGluZ0MBEjUAAAEAAAAPAAAAB0N1bGxpbmdTCgAAAEN1bGxpbmdPZmYAAAAAAAAAAAAAAAAApDgAAAMAAAAlAAAACE1hdGVyaWFsTL/t+yoAAAAAUxIAAABNYXRlcmlhbAABTWF0ZXJpYWxTAAAAAHI1AAABAAAABQAAAAdWZXJzaW9uSWYAAACVNQAAAQAAAAoAAAAMU2hhZGluZ01vZGVsUwUAAABQaG9uZ7E1AAABAAAABQAAAApNdWx0aUxheWVySQAAAACXOAAAAAAAAAAAAAAMUHJvcGVydGllczcwGTYAAAcAAABBAAAAAVBTDAAAAERpZmZ1c2VDb2xvclMFAAAAQ29sb3JTAAAAAFMBAAAAQUQAAACgmZnpP0QAAACgmZnpP0QAAACgmZnpP2g2AAAHAAAAQQAAAAFQUwwAAABBbWJpZW50Q29sb3JTBQAAAENvbG9yUwAAAABTAQAAAEFEAAAAQG4Mqj9EAAAAQG4Mqj9EAAAAQG4Mqj+nNgAABQAAADEAAAABUFMNAAAAQW1iaWVudEZhY3RvclMGAAAATnVtYmVyUwAAAABTAQAAAEFEAAAAAAAAAADoNgAABQAAADMAAAABUFMKAAAAQnVtcEZhY3RvclMGAAAAZG91YmxlUwYAAABOdW1iZXJTAAAAAEQAAAAAAAAAADg3AAAHAAAAQgAAAAFQUw0AAABTcGVjdWxhckNvbG9yUwUAAABDb2xvclMAAAAAUwEAAABBRAAAAKCZmek/RAAAAKCZmek/RAAAAKCZmek/eDcAAAUAAAAyAAAAAVBTDgAAAFNwZWN1bGFyRmFjdG9yUwYAAABOdW1iZXJTAAAAAFMBAAAAQUQAAAAAAADQP7M3AAAFAAAALQAAAAFQUwkAAABTaGluaW5lc3NTBgAAAE51bWJlclMAAAAAUwEAAABBRAAAAAAAADlA9jcAAAUAAAA1AAAAAVBTEQAAAFNoaW5pbmVzc0V4cG9uZW50UwYAAABOdW1iZXJTAAAAAFMBAAAAQUQAAAAAAAA5QEg4AAAHAAAARAAAAAFQUw8AAABSZWZsZWN0aW9uQ29sb3JTBQAAAENvbG9yUwAAAABTAQAAAEFEAAAAoJmZ6T9EAAAAoJmZ6T9EAAAAoJmZ6T+KOAAABQAAADQAAAABUFMQAAAAUmVmbGVjdGlvbkZhY3RvclMGAAAATnVtYmVyUwAAAABTAQAAAEFEAAAAAAAAAAAAAAAAAAAAAAAAAAAAAAAAAAAAAAAAAAAAAAAAAAAAAAAAAAAAAABLOQAAAAAAAAAAAAALQ29ubmVjdGlvbnPwOAAAAwAAABkAAAABQ1MCAAAAT09MpbHxGQAAAABMAAAAAAAAAAAXOQAAAwAAABkAAAABQ1MCAAAAT09Mzxw0BwAAAABMpbHxGQAAAAA+OQAAAwAAABkAAAABQ1MCAAAAT09Mv+37KgAAAABMpbHxGQAAAAAAAAAAAAAAAAAAAAAAgzkAAAAAAAAAAAAABVRha2VzdjkAAAEAAAAFAAAAB0N1cnJlbnRTAAAAAAAAAAAAAAAAAAAAAAAAAAAAAAAAAAAAAAAA+ryrCdDI1GaxdvuDHPcmfgAAAAAAAAAAAAAAAAAAAADoHAAAAAAAAAAAAAAAAAAAAAAAAAAAAAAAAAAAAAAAAAAAAAAAAAAAAAAAAAAAAAAAAAAAAAAAAAAAAAAAAAAAAAAAAAAAAAAAAAAAAAAAAAAAAAAAAAAAAAAAAAAAAAAAAAAAAAAAAAAAAAAAAAAAAAAAAAAAAAAAAAAA+FqMat712X7s6QzjdY8pCw==" (`self.Mesh`))
  (`SceneComponent.SetWorldScale3D` _mesh (50.0 50.0 50.0))
  (`SceneComponent.K2_AddWorldOffset` _mesh (0.0 0.0 500.0) false false))

(fn `UserConstructionScript`)