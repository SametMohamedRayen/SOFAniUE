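; Non-AR pawn that turns horizontal touch swipes into SwipeLeft and SwipeRight event dispatcher calls.
; Touch press records the start point; Tick then checks a distance threshold and compares axes to pick a direction, ignoring mostly vertical movement.
; A DoOnce gate, reset on release, limits evaluation to once per touch.
; The threshold reads TouchEnd before refreshing it from live touch state, and IsPressed is never cleared.
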(event `self.ReceiveTick`
  (params (DeltaSeconds :type "Float (single-precision)"))
  (bind (_locationx _locationy) (`PlayerController.GetInputTouchState` (`GameplayStatics.GetPlayerController` 0) "Touch1"))
  (bind (_x _y) (`KismetMathLibrary.BreakVector2D` (- (`self.TouchStart`) (`self.TouchEnd`))))
  (if (`self.IsPressed`)
    (if (> (`KismetMathLibrary.VSize2D` (- (`self.TouchStart`) (`self.TouchEnd`))) 100.0)
      (`/Engine/EditorBlueprintResources/StandardMacros.DoOnce` false :!label _label
        (:`Completed`
          (set `self.TouchEnd` (`KismetMathLibrary.MakeVector2D` _locationx _locationy))
          (if (> (`KismetMathLibrary.Abs` _x) (`KismetMathLibrary.Abs` _y))
            (if (> _x 0.0)
              (`self.SwipeLeftEventDispatcher`)
              (else
                (`self.SwipeRightEventDispatcher`)))))))))

(event `InputTouch`
  (params (Location :type "Vector Structure") (FingerIndex :type "ETouchIndex Enum"))
  (:`Pressed`
    (set `self.IsPressed` true)
    (set `self.TouchStart` (`KismetMathLibrary.MakeVector2D` Location_X Location_Y)))
  (:`Released`
    (set `self.TouchEnd` (`KismetMathLibrary.MakeVector2D` Location_X Location_Y))
    (goto _label :!via `Reset`)))

(fn `UserConstructionScript`)