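; Pagination helper that splits a flat item array into fixed-size pages, with next/previous page lookups and debug printing of item names.
; CreatePagesOfItems computes page count and each page's last index, mapping page slots to flat array indices.
; One working array is reused: filled on the first page, overwritten on middle pages, rebuilt on the last.
; That rebuild's reset uses a hard-coded removal count, independent of page size.
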(fn `CreatePagesOfItems`
  (params (ArrayOfItems :type "Array of ItemEntity Structure") (SizeOfPage :type Integer))
  (returns (ArrayOfPages :type "Array of /Game/InventoryFeature/DataStructures/Page_S Structure"))
  (locals (PagesCount :type Integer) (CurrentPageIndex :type Integer) (LastItemInPageIndex :type Integer) (CurrentPageItems :type "Array of ItemEntity Structure") (ItemsPages :type "Array of /Game/InventoryFeature/DataStructures/Page_S Structure"))
  (bind _returnvalue (`KismetArrayLibrary.Array_Length` ArrayOfItems))
  (bind _currentpageitems (`local.CurrentPageItems`))
  (bind _returnvalue_2 (- (`local.PagesCount`) 1))
  (bind _returnvalue_3 (mod (`KismetArrayLibrary.Array_Length` (`local.ArrayOfItems`)) (`local.SizeOfPage`)))
  (if (== _returnvalue 0)
    (set `local.PagesCount` 0)
    (else
      (set `local.PagesCount` (+ (/ _returnvalue SizeOfPage) (!= (mod _returnvalue SizeOfPage) 0)))))
  (for _index (range (+ _returnvalue_2 1))
    (bind _output_get (set `local.CurrentPageIndex` _index))
    (bind _returnvalue_4 (== _output_get _returnvalue_2))
    (if _returnvalue_4
      (for _ (range 4)
        (`KismetArrayLibrary.Array_Remove` (`local.CurrentPageItems`))))
    (if (== (- (`local.PagesCount`) 1) _output_get)
      (if (!= _returnvalue_3 0)
        (set `local.LastItemInPageIndex` (- _returnvalue_3 1))
        (else
          (set `local.LastItemInPageIndex` (- (`local.SizeOfPage`) 1) :!label _label)))
      (else
        (goto _label)))
    (for _index_2 (range (+ (`local.LastItemInPageIndex`) 1))
      (if (or (== _output_get 0) _returnvalue_4)
        (bind _output (`|GetArrayItem` (`local.ArrayOfItems`) (+ _index_2 (* _output_get (`local.SizeOfPage`)))))
        (`KismetArrayLibrary.Array_Add` _currentpageitems _output)
        (else
          (`KismetArrayLibrary.Array_Set` _currentpageitems _index_2 _output))))
    (`KismetArrayLibrary.Array_Add` (`local.ItemsPages`) (make `/Game/InventoryFeature/DataStructures/Page_S` (`local.CurrentPageItems`))))
  (return (`local.ItemsPages`)))

(fn `NextPage`
  (params (CurrentPageIndex :type Integer) (ItemsPages :type "Array of /Game/InventoryFeature/DataStructures/Page_S Structure"))
  (returns (NextPage :type "/Game/InventoryFeature/DataStructures/Page_S Structure") (NextPageIndex :type Integer))
  (locals (LastPageIndex :type Integer))
  (bind _returnvalue (+ (`local.CurrentPageIndex`) 1))
  (bind _output_get (set `local.LastPageIndex` (- (`KismetArrayLibrary.Array_Length` ItemsPages) 1)))
  (if (!= _output_get CurrentPageIndex)
    (return (`|GetArrayItem` (`local.ItemsPages`) _returnvalue) _returnvalue)))

(fn `PreviousPage`
  (params (CurrentPageIndex :type Integer) (ItemsPages :type "Array of /Game/InventoryFeature/DataStructures/Page_S Structure"))
  (returns (PreviousPage :type "/Game/InventoryFeature/DataStructures/Page_S Structure") (PreviousPageIndex :type Integer))
  (bind _returnvalue (- CurrentPageIndex 1))
  (if (!= CurrentPageIndex 0)
    (return (`|GetArrayItem` ItemsPages _returnvalue) _returnvalue)))

(fn `PrintItems`
  (params (ItemsArray :type "Array of ItemEntity Structure"))
  (for _array_element ItemsArray
    (`KismetSystemLibrary.PrintString` null (`.Name` (break `ItemEntity` _array_element)))))

(fn `PrintPages`
  (params (ItemsPages :type "Array of /Game/InventoryFeature/DataStructures/Page_S Structure"))
  (for (_array_element _array_index) ItemsPages
    (`self.PrintItems` (`.PageItems_3_CDDDE1BA4992C0E32A32DB93AA63CC47` (break `/Game/InventoryFeature/DataStructures/Page_S` _array_element)))))